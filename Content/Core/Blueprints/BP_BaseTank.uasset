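; Player-controlled base tank that moves along world axes from input and fires missiles on left click.
; Each movement input applies a swept offset, snaps the Hull relative to its starting yaw and sets MissileDirection.
; Forward/backward input also adds rotation to the top-down camera and sets flags that halve rightward speed on diagonals; leftward speed is unadjusted.
; Clicking spawns a BP_BaseMissile at MissileSpawnPlace and passes it MissileDirection.
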(event `InputAxis|MoveForward`
  (params (AxisValue :type "Float (single-precision)"))
  (bind (_initialtankrotation_roll _initialtankrotation_pitch _initialtankrotation_yaw) (`KismetMathLibrary.BreakRotator` (`self.InitialTankRotation`)))
  (bind (_initialtankrotation_roll_2 _initialtankrotation_pitch_2 _initialtankrotation_yaw_2) (`KismetMathLibrary.BreakRotator` (`self.InitialTankRotation`)))
  (if (> AxisValue 0.0)
    (`self.K2_AddActorWorldOffset` (0.0 4.0 0.0) true)
    (`SceneComponent.K2_SetWorldRotation` (`self.Hull`) (`KismetMathLibrary.MakeRotator` 0.0 0.0 _initialtankrotation_yaw_2) false false)
    (set `self.MissileDirection` (0.0 100.0 0.0))
    (set `self.IsForwardMoving` true)
    (`SceneComponent.K2_AddWorldRotation` (`self.TopDownCamera`) (`KismetMathLibrary.MakeRotator` _initialtankrotation_roll _initialtankrotation_pitch _initialtankrotation_yaw) false false)
    (else
      (set `self.IsForwardMoving` false))))

(event `InputAxis|MoveForward`
  (params (AxisValue :type "Float (single-precision)"))
  (bind (_initialtankrotation_roll _initialtankrotation_pitch _initialtankrotation_yaw) (`KismetMathLibrary.BreakRotator` (`self.InitialTankRotation`)))
  (bind (_initialtankrotation_roll_2 _initialtankrotation_pitch_2 _initialtankrotation_yaw_2) (`KismetMathLibrary.BreakRotator` (`self.InitialTankRotation`)))
  (if (< AxisValue 0.0)
    (`self.K2_AddActorWorldOffset` (0.0 -4.0 0.0) true)
    (`SceneComponent.K2_SetWorldRotation` (`self.Hull`) (`KismetMathLibrary.MakeRotator` 0.0 0.0 (- _initialtankrotation_yaw_2 180.0)) false false)
    (set `self.MissileDirection` (0.0 -100.0 0.0))
    (set `self.IsBackwardMoving` true)
    (`SceneComponent.K2_AddWorldRotation` (`self.TopDownCamera`) (`KismetMathLibrary.MakeRotator` _initialtankrotation_roll _initialtankrotation_pitch (- _initialtankrotation_yaw 180.0)) false false)
    (else
      (set `self.IsBackwardMoving` false))))

(event `InputAxis|MoveRight`
  (params (AxisValue :type "Float (single-precision)"))
  (bind (_initialtankrotation_roll _initialtankrotation_pitch _initialtankrotation_yaw) (`KismetMathLibrary.BreakRotator` (`self.InitialTankRotation`)))
  (if (> AxisValue 0.0)
    (if (or (`self.IsForwardMoving`) (`self.IsBackwardMoving`))
      (set `self.MoveRightSpeed` (/ (`self.MoveRightSpeed`) 2.0))
      (set `self.IsDiagonallyRightMoving` true)
      (elif (`self.IsDiagonallyRightMoving`)
        (set `self.MoveRightSpeed` (* (`self.MoveRightSpeed`) 2.0))
        (set `self.IsDiagonallyRightMoving` false)))
    (`self.K2_AddActorWorldOffset` (`KismetMathLibrary.MakeVector` (`self.MoveRightSpeed`)) true)
    (`SceneComponent.K2_SetWorldRotation` (`self.Hull`) (`KismetMathLibrary.MakeRotator` 0.0 0.0 (+ _initialtankrotation_yaw 90.0)) false false)
    (set `self.MissileDirection` (-100.0 0.0 0.0))))

(event `InputAxis|MoveRight`
  (params (AxisValue :type "Float (single-precision)"))
  (bind (_initialtankrotation_roll _initialtankrotation_pitch _initialtankrotation_yaw) (`KismetMathLibrary.BreakRotator` (`self.InitialTankRotation`)))
  (if (< AxisValue 0.0)
    (`self.K2_AddActorWorldOffset` (`KismetMathLibrary.MakeVector` (`self.MoveLeftSpeed`)) true)
    (`SceneComponent.K2_SetWorldRotation` (`self.Hull`) (`KismetMathLibrary.MakeRotator` 0.0 0.0 (- _initialtankrotation_yaw 90.0)) false false)
    (set `self.MissileDirection` (100.0 0.0 0.0))))

(event `self.ReceiveBeginPlay`
  (set `self.InitialTankRotation` (`SceneComponent.K2_GetComponentRotation` (`self.Hull`)))
  (set `self.InitialTopDownCameraRotation` (`SceneComponent.K2_GetComponentRotation` (`self.TopDownCamera`))))

(event `Key|LeftMouseButton`
  (params (Key :type "Key Structure"))
  (:`Pressed`
    (bind _returnvalue (`|SpawnActorFromClass` "/Game/Core/Blueprints/BP_BaseMissile.BP_BaseMissile_C" (`KismetMathLibrary.MakeTransform` (`SceneComponent.K2_GetComponentLocation` (`self.MissileSpawnPlace`)) (struct) (`self.SpawnTransformScaleMissile`)) "AlwaysSpawn" "OverrideRootScale" null null))
    (set `/Game/Core/Blueprints/BP_BaseMissile.Direction` (`self.MissileDirection`) _returnvalue)))

(fn `UserConstructionScript`)
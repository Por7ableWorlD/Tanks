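; Destructible wall actor that is destroyed when a tank (BP_BaseTank) begins overlapping it.
; On Hit it calls the parent handler, then switches the Wall component's material to BasicAsset03 if the other actor is a BP_BaseMissile, so missiles only change its look.
; Tick is empty, and leftover material and debug-print nodes are disconnected.
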(event `self.ReceiveTick`
  (params (DeltaSeconds :type "Float (single-precision)")))

(event `self.ReceiveActorBeginOverlap`
  (params (OtherActor :type "Actor Object Reference"))
  (cast `/Game/Core/Blueprints/BP_BaseTank` OtherActor)
  (`self.K2_DestroyActor`))

(event `self.ReceiveHit`
  (params (MyComp :type "PrimitiveComponent Object Reference") (Other :type "Actor Object Reference") (OtherComp :type "PrimitiveComponent Object Reference") (bSelfMoved :type Boolean) (HitLocation :type "Vector Structure") (HitNormal :type "Vector Structure") (NormalImpulse :type "Vector Structure") (Hit :type "HitResult Structure (by ref)"))
  (set `self.MyComp` MyComp)
  (bind _output_get (set `self.Other` Other))
  (`parent.ReceiveHit` (`self.MyComp`) _output_get OtherComp bSelfMoved HitLocation HitNormal NormalImpulse Hit)
  (`self.MyComp`
    (:`then`
      (cast `/Game/Core/Blueprints/BP_BaseMissile` (`self.Other`))
      (`PrimitiveComponent.SetMaterial` (`self.Wall`) 0 "/Engine/MapTemplates/Materials/BasicAsset03.BasicAsset03"))
    (:`else`)))

(fn `UserConstructionScript`
  (`parent.UserConstructionScript`))